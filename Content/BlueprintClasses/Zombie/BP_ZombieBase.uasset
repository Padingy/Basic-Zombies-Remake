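; BP_ZombieBase is a zombie Blueprint that provides a melee attack against BP_ZombiesCharacter pawns.
; MeleeAttack plays the ZombieAttack montage, and its notify begin triggers a sphere overlap at the Sphere component's location and radius.
; Each overlapped character takes Damage, credited to the zombie and its controller, and a debug sphere is drawn to show the hit area.
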(event `Melee Attack`
  (bind _returnvalue (`SceneComponent.K2_GetComponentLocation` (`self.Sphere`)))
  (bind _returnvalue_2 (`SphereComponent.GetScaledSphereRadius` (`self.Sphere`)))
  (`|PlayMontage` (`self.Mesh`) "/Game/BlueprintClasses/Zombie/Animations/ZombieAttack.ZombieAttack"
    (:`OnNotifyBegin`
      (bind _outactors (`KismetSystemLibrary.SphereOverlapActors` _returnvalue _returnvalue_2 (`|MakeArray` "ObjectTypeQuery3" :!type "EObjectTypeQuery Enum") "/Game/BlueprintClasses/Player/BP_ZombiesCharacter.BP_ZombiesCharacter_C" (`|MakeArray` self :!type "Actor Object Reference")))
      (`KismetSystemLibrary.DrawDebugSphere` _returnvalue _returnvalue_2 12 (struct :`G` 1.0 :`B` 0.049809 :`A` 1.0) 10.0)
      (for _array_element _outactors
        (`GameplayStatics.ApplyDamage` _array_element (`self.damage`) (`self.GetController`) self)))))

(fn `UserConstructionScript`)