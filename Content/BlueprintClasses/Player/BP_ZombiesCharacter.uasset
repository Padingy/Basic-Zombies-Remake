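; Player character Blueprint for a zombies game that owns the HUD, pause and death screens and scales look input.
; BeginPlay creates and stores the HUD, and the DeathScreen event swaps it for the death widget, disables movement and switches to UI-only input.
; The Pause action reuses a cached pause widget to toggle game pause, swapping widgets, cursor visibility and input mode.
; Turn and LookUp axes are multiplied by a Sensitivity variable.
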(event `self.ReceiveBeginPlay`
  ;[1 1 1] BeginPlay - Make HUD
  (bind _returnvalue (`|CreateWidget` "/Game/BlueprintClasses/Player/HUD/HUD_Widget.HUD_Widget_C"))
  (bind _output_get (set `self.HUD WIdget REF` _returnvalue))
  (`UserWidget.AddToViewport` _output_get 0))

(event `self.DeathScreen`
  (bind _returnvalue (`GameplayStatics.GetPlayerController` 0))
  ;[1 1 1] Death Event
  (bind _foundwidgets (`WidgetBlueprintLibrary.GetAllWidgetsOfClass` "/Game/BlueprintClasses/Player/HUD/HUD_Widget.HUD_Widget_C"))
  (for _array_element _foundwidgets
    (`Widget.RemoveFromParent` _array_element)
    (bind _returnvalue_2 (`|CreateWidget` "/Game/BlueprintClasses/Player/HUD/Death_Screen.Death_Screen_C"))
    (`UserWidget.AddToViewport` _returnvalue_2 0)
    (`CharacterMovementComponent.DisableMovement` (`self.CharacterMovement`))
    (set `PlayerController.bShowMouseCursor` true _returnvalue)
    (`WidgetBlueprintLibrary.SetInputMode_UIOnlyEx` _returnvalue null)))

(event `InputAction|Pause` :paused true
  (params (Key :type "Key Structure"))
  (bind _returnvalue (`GameplayStatics.GetPlayerController` 0))
  (bind _returnvalue_2 (`GameplayStatics.GetPlayerController` 0))
  (bind _pause_widget_ref (`self.Pause Widget REF`))
  ;[1 1 1] Pause Menu
  (:`Pressed`
    (`/Engine/EditorBlueprintResources/StandardMacros.IsValid` (`self.Pause Widget REF`)
      (:`Is Valid`
        _)
      (:`Is Not Valid`
        (bind _returnvalue_3 (`|CreateWidget` "/Game/BlueprintClasses/Player/HUD/Pause_Widget.Pause_Widget_C"))
        (set `self.Pause Widget REF` _returnvalue_3)))
    (if (`GameplayStatics.IsGamePaused`)
      (`WidgetLayoutLibrary.RemoveAllWidgets`)
      (`GameplayStatics.SetGamePaused` false)
      (`UserWidget.AddToViewport` (`self.HUD WIdget REF`) 0)
      (set `PlayerController.bShowMouseCursor` false _returnvalue_2)
      (`WidgetBlueprintLibrary.SetInputMode_GameOnly` _returnvalue_2)
      (else
        (bind _foundwidgets (`WidgetBlueprintLibrary.GetAllWidgetsOfClass` "/Game/BlueprintClasses/Player/HUD/HUD_Widget.HUD_Widget_C"))
        (for _array_element _foundwidgets
          (`Widget.RemoveFromParent` _array_element)
          (`UserWidget.AddToViewport` _pause_widget_ref 0)
          (`GameplayStatics.SetGamePaused` true)
          (set `PlayerController.bShowMouseCursor` true _returnvalue)
          (`WidgetBlueprintLibrary.SetInputMode_GameAndUIEx` _returnvalue _pause_widget_ref "DoNotLock" false))))))

(event `InputAxis|Turn`
  (params (AxisValue :type "Float (single-precision)"))
  ;[1 1 1] Sensitivity
  (`self.AddControllerYawInput` (* AxisValue (`self.sensitivity`))))

(event `InputAxis|LookUp`
  (params (AxisValue :type "Float (single-precision)"))
  ;[1 1 1] Sensitivity
  (`self.AddControllerPitchInput` (* AxisValue (`self.sensitivity`))))

(fn `UserConstructionScript`)